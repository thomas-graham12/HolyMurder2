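; Zombie enemy AI that wanders, chases the player on sight and deals contact damage.
; Tick issues delayed moves to random nearby reachable points while CanSeePlayer is false; PawnSensing starts the chase, and a retriggerable delay clears the flag when sightings stop.
; Projectile overlaps reduce EnemyHealth until the actor is destroyed.
; Capsule hits lower player Health through a DoOnce gate, which resets after a short delay only following a player hit.
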(event `self.ReceiveActorBeginOverlap`
  (params (OtherActor :type "Actor Object Reference"))
  (cast `/Game/FirstPerson/Blueprints/BP_FirstPersonProjectile` OtherActor)
  (set `self.EnemyHealth` (- (`self.EnemyHealth`) 0.5))
  (if (<= (`self.EnemyHealth`) 0.0)
    (`self.K2_DestroyActor`)))

(event `self.ReceiveTick`
  (params (DeltaSeconds :type "Float (single-precision)"))
  ;[1 1 1] Random Patrol if cannot see player
  (if (not (`self.Can See Player?`))
    (`KismetSystemLibrary.Delay` (`KismetMathLibrary.RandomFloatInRange` 3.0 5.0))
    (`|AIMoveTo` self (`NavigationSystemV1.K2_GetRandomReachablePointInRadius` (`self.K2_GetActorLocation`) 500.0 null null) null)))

(event `self.PawnSensing.OnSeePawn`
  (params (Pawn :type "Pawn Object Reference"))
  ;[1 1 1] Chase Player
  (bind _asbp_first_person_character (cast `/Game/FirstPerson/Blueprints/BP_FirstPersonCharacter` Pawn))
  (`|ExecutionSequence`
    (:`then_0`
      (set `self.Can See Player?` true)
      (`|AIMoveTo` self (0.0 0.0 0.0) _asbp_first_person_character))
    (:`then_1`
      (`KismetSystemLibrary.RetriggerableDelay` 0.5)
      (set `self.Can See Player?` false))))

(event `self.CapsuleComponent.OnComponentHit`
  (params (HitComponent :type "PrimitiveComponent Object Reference") (OtherActor :type "Actor Object Reference") (OtherComp :type "PrimitiveComponent Object Reference") (NormalImpulse :type "Vector Structure") (Hit :type "HitResult Structure (by ref)"))
  (`/Engine/EditorBlueprintResources/StandardMacros.DoOnce` false :!label _label
    (:`Completed`
      (bind _asbp_first_person_character (cast `/Game/FirstPerson/Blueprints/BP_FirstPersonCharacter` OtherActor))
      (set `/Game/FirstPerson/Blueprints/BP_FirstPersonCharacter.Health` (- (`/Game/FirstPerson/Blueprints/BP_FirstPersonCharacter.Health` _asbp_first_person_character) 0.25) _asbp_first_person_character)
      (`KismetSystemLibrary.Delay` 0.3)
      (goto _label :!via `Reset`))))

(fn `UserConstructionScript`)